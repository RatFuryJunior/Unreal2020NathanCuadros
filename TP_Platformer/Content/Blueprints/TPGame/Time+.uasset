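; Time pickup actor that notifies the HUD when collected.
; On any actor overlap, it casts the first player's HUD to TPGamehud, calls TimeCollected, then destroys itself.
; The construction script applies a configurable mesh to the Cylinder component and sets the rotating movement's rate, pivot and local-space option from variables.
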(event EventBeginPlay)

(event Collision|EventActorBeginOverlap
  (params (OtherActor :type Actor%20Object%20Reference))
  (bind _astpgamehud (Utilities|Casting|CastToTPGamehud (HUD|GetHUD (Game|GetPlayerController 0))))
  (Default|TimeCollected _astpgamehud)
  (Actor|DestroyActor))

(event EventTick
  (params (DeltaSeconds :type Float%20%28single-precision%29)))

(fn ConstructionScript
  (bind _rotatingmovement (Variables|Default|GetRotatingMovement))
  (Components|StaticMesh|SetStaticMesh (Variables|Default|GetCylinder) (Variables|Default|GetMesh))
  (Variables|/Script/Engine.RotatingMovementComponent|SetRotationRate _rotatingmovement (Variables|Default|GetRotation%20Rated))
  (Variables|/Script/Engine.RotatingMovementComponent|SetPivotTranslation _rotatingmovement (Variables|Default|GetPivot%20Translation))
  (Variables|/Script/Engine.RotatingMovementComponent|SetbRotationInLocalSpace _rotatingmovement (Variables|Default|GetRotation%20in%20location)))